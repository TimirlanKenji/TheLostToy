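; BP_YippyCharacter is a child character Blueprint that adds a RotatingMovement component toggle to its parent's death and run-start logic.
; Death calls the parent, activates the rotation, sets a one-second timer with no function name, then deactivates the rotation immediately.
; SrartRun calls the parent and switches rotation off, while BeginPlay, Tick and the construction script only forward to the parent.
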(event EventBeginPlay
  (|CallParentFunction))

(event Collision|EventActorBeginOverlap
  (params (OtherActor :type Actor%20Object%20Reference)))

(event EventTick
  (params (DeltaSeconds :type Float%20%28single-precision%29))
  (|CallParentFunction 0.0))

(fn ConstructionScript
  (|CallParentFunction))

(fn Death
  (bind _rotatingmovement (Variables|Default|GetRotatingMovement))
  (|CallParentFunction)
  (Components|Activation|Activate _rotatingmovement true)
  (Utilities|Time|SetTimerbyFunctionName _rotatingmovement "" 1.0)
  (Components|Activation|Deactivate _rotatingmovement))

(fn SrartRun
  (|CallParentFunction)
  (Components|Activation|Deactivate (Variables|Default|GetRotatingMovement)))