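; AI controller that, on possess, picks patrol-chase or random-wander behavior from the enemy character's type.
; Patrol-chase follows the pawn's spline points in a loop, advancing on move success or failure and checking player distance before each move.
; When the player is close, it moves toward them and re-checks after a short delay.
; Random enemies use a looping timer to walk to random reachable points around themselves.
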(event Custom|WalkRandom
  (AI|AIMoveTo (Pawn|GetControlledPawn) (.RandomLocation (AI|Navigation|GetRandomReachablePointinRadius (Transformation|GetActorLocation (Pawn|GetControlledPawn)) 5e+03 0 0)) 0 5.0 false))

(event Custom|PatrolChase
  (bind _enemypatrolchase (Variables|Default|GetEnemyPatrolChase))
  ;[1 1 1] EnemyPatrolChase logic
  (if (<= (Transformation|GetDistanceTo (Pawn|GetControlledPawn) (Game|GetPlayerCharacter 0)) 5e+02)
    (AI|AIMoveTo (Pawn|GetControlledPawn) "0, 0, 0" (Game|GetPlayerCharacter 0) 5.0 false
      (:then
        (Utilities|FlowControl|Delay 2.0)
        (CallFunction|PatrolChase)))
    (else
      (AI|AIMoveTo (Variables|Default|GetEnemyPatrolChase) (Spline|GetLocationatSplinePoint (Variables|/Game/Blueprints/Enemy/BP_EnemyCharacter.BP_EnemyCharacter_C|GetPath _enemypatrolchase) (Variables|/Game/Blueprints/Enemy/BP_EnemyCharacter.BP_EnemyCharacter_C|GetSplineIndex _enemypatrolchase) "World") 0 2.0 false
        (:OnSuccess
          _)
        (:OnFail
          _))
      (if (== (Variables|/Game/Blueprints/Enemy/BP_EnemyCharacter.BP_EnemyCharacter_C|GetSplineIndex _enemypatrolchase) (Variables|/Game/Blueprints/Enemy/BP_EnemyCharacter.BP_EnemyCharacter_C|GetMaxSplinePoints (Variables|Default|GetEnemyPatrolChase)))
        (Variables|/Game/Blueprints/Enemy/BP_EnemyCharacter.BP_EnemyCharacter_C|SetSplineIndex (Variables|Default|GetEnemyPatrolChase) 0)
        (else
          (Math|Integer|IncrementInt (Variables|/Game/Blueprints/Enemy/BP_EnemyCharacter.BP_EnemyCharacter_C|GetSplineIndex (Variables|Default|GetEnemyPatrolChase))
            (:%20%20
              _))))
      (CallFunction|PatrolChase))))

(event EventPossess
  (params (PossessedPawn :type Pawn%20Object%20Reference))
  (switch Utilities|FlowControl|Switch|SwitchonENUM_EnemyType (Variables|/Game/Blueprints/Enemy/BP_EnemyCharacter.BP_EnemyCharacter_C|GetEnemyType (.AsBP%20Enemy%20Character (Utilities|Casting|CastToBP_EnemyCharacter (Pawn|GetControlledPawn))))
    (:NewEnumerator2
      (bind _asbp_enemy_patrol_chase (Utilities|Casting|CastToBP_Enemy_PatrolChase (Pawn|GetControlledPawn)))
      (Variables|Default|SetEnemyPatrolChase _asbp_enemy_patrol_chase)
      (CallFunction|PatrolChase))
    (:NewEnumerator3
      (bind _asbp_enemy_random (Utilities|Casting|CastToBP_EnemyRandom (Pawn|GetControlledPawn)))
      (Variables|Default|SetBP_EnemyRandom _asbp_enemy_random)
      (Utilities|Time|SetTimerbyFunctionName 0 "WalkRandom" 3.0 true))))

(fn ConstructionScript)