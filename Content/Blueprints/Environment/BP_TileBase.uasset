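; Base track tile for an endless runner that extends the path as the player character passes through it.
; Two trigger boxes each fire once, asking the game mode to spawn another tile and adding multiplied points.
; Only the first box also raises walk speed, up to a clamp.
; BeginPlay calls an empty SpawnObstacle, leaving the random obstacle and plushe spawner unwired, and the delayed self-destroy is likewise disconnected.
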(event OnComponentBeginOverlap(Box1)
  (params (OverlappedComponent :type Primitive%20Component%20Object%20Reference) (OtherActor :type Actor%20Object%20Reference) (OtherComp :type Primitive%20Component%20Object%20Reference) (OtherBodyIndex :type Integer) (bFromSweep :type Boolean) (SweepResult :type Hit%20Result%20Structure%20%28by%20ref%29))
  (Utilities|Casting|CastToBP_ThirdPersonCharacter OtherActor)
  (Utilities|FlowControl|DoOnce false
    (:Completed
      (bind _asbp_third_person_game_mode (Utilities|Casting|CastToBP_ThirdPersonGameMode (Game|GetGameMode)))
      (Default|SpawnTile _asbp_third_person_game_mode "BP_TileBase_C")
      ;[1 1 1] Points logic
      (Variables|/Game/Blueprints/BP_ThirdPersonGameMode.BP_ThirdPersonGameMode_C|SetCurrentPoints _asbp_third_person_game_mode (+ (Variables|/Game/Blueprints/BP_ThirdPersonGameMode.BP_ThirdPersonGameMode_C|GetCurrentPoints _asbp_third_person_game_mode) (* 1 (Variables|/Game/Blueprints/BP_ThirdPersonGameMode.BP_ThirdPersonGameMode_C|GetPointsMultiplier _asbp_third_person_game_mode)))))))

(event OnComponentBeginOverlap(Box)
  (params (OverlappedComponent :type Primitive%20Component%20Object%20Reference) (OtherActor :type Actor%20Object%20Reference) (OtherComp :type Primitive%20Component%20Object%20Reference) (OtherBodyIndex :type Integer) (bFromSweep :type Boolean) (SweepResult :type Hit%20Result%20Structure%20%28by%20ref%29))
  (Utilities|Casting|CastToBP_ThirdPersonCharacter OtherActor)
  (Utilities|FlowControl|DoOnce false
    (:Completed
      (bind _asbp_third_person_game_mode (Utilities|Casting|CastToBP_ThirdPersonGameMode (Game|GetGameMode)))
      (Default|SpawnTile _asbp_third_person_game_mode "BP_TileBase_C")
      ;[1 1 1] Points logic
      (Variables|/Game/Blueprints/BP_ThirdPersonGameMode.BP_ThirdPersonGameMode_C|SetCurrentPoints _asbp_third_person_game_mode (+ (Variables|/Game/Blueprints/BP_ThirdPersonGameMode.BP_ThirdPersonGameMode_C|GetCurrentPoints _asbp_third_person_game_mode) (* 1 (Variables|/Game/Blueprints/BP_ThirdPersonGameMode.BP_ThirdPersonGameMode_C|GetPointsMultiplier _asbp_third_person_game_mode))))
      ;[1 0 0.6878] SpeedUp logic (from 600 to 2500 !!)
      (bind _asbp_third_person_character (Utilities|Casting|CastToBP_ThirdPersonCharacter (Game|GetPlayerCharacter 0)))
      (Variables|/Script/Engine.CharacterMovementComponent|SetMaxWalkSpeed (Variables|/Script/Engine.Character|GetCharacterMovement _asbp_third_person_character) (Math|Float|Clamp(Float) (* (Variables|/Script/Engine.CharacterMovementComponent|GetMaxWalkSpeed (Variables|/Script/Engine.Character|GetCharacterMovement _asbp_third_person_character)) 1.2) 6e+02 1.5e+03)))))

(event EventBeginPlay
  (CallFunction|SpawnObstacle))

(event Collision|EventActorBeginOverlap
  (params (OtherActor :type Actor%20Object%20Reference)))

(event EventTick
  (params (DeltaSeconds :type Float%20%28single-precision%29)))

(fn ConstructionScript)

(fn SpawnObstacle)

(fn RandomSpawnObstacle
  (params (InTransform :type Transform))
  (switch int (Math|Random|RandomIntegerinRange 0 (Variables|Default|GetMaxRandomObstacleID))
    (:2
      (bind _returnvalue (Game|SpawnActorfromClass "/Game/Blueprints/Environment/BP_Obstacle_A.BP_Obstacle_A_C" InTransform "Undefined" 0 0))
      (Utilities|Array|AddUnique (Variables|Default|GetObstacles) _returnvalue))
    (:3
      (bind _returnvalue_2 (Game|SpawnActorfromClass "/Game/Blueprints/Environment/BP_Obstacle_B.BP_Obstacle_B_C" InTransform "Undefined" 0 0))
      (Utilities|Array|AddUnique (Variables|Default|GetObstacles) _returnvalue_2))
    (:4
      (Game|SpawnActorfromClass "/Game/Blueprints/Environment/BP_Plushe.BP_Plushe_C" InTransform "Undefined" 0 0)
      (Utilities|Array|AddUnique (Variables|Default|GetObstacles) 0))))