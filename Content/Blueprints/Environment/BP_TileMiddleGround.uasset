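; BP_TileMiddleGround is a middle-ground environment tile that dresses itself with random forest decor and chains into the next tile.
; On BeginPlay, RandomSpawnDecor scatters trees, stumps, bark and vegetation across TileFloorA, B and D as hierarchical instanced meshes.
; Helpers pick random points within each floor's bounds, with random yaw and uniform scale.
; When the player first overlaps the Box, the game mode's SpawnMiddleGround is called and the tile destroys itself after a short delay.
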(event OnComponentBeginOverlap(Box)
  (params (OverlappedComponent :type Primitive%20Component%20Object%20Reference) (OtherActor :type Actor%20Object%20Reference) (OtherComp :type Primitive%20Component%20Object%20Reference) (OtherBodyIndex :type Integer) (bFromSweep :type Boolean) (SweepResult :type Hit%20Result%20Structure%20%28by%20ref%29))
  (Utilities|Casting|CastToBP_ThirdPersonCharacter OtherActor)
  (Utilities|FlowControl|DoOnce false
    (:Completed
      (bind _asbp_third_person_game_mode (Utilities|Casting|CastToBP_ThirdPersonGameMode (Game|GetGameMode)))
      (Default|SpawnMiddleGround _asbp_third_person_game_mode "BP_TileMiddleGround_C")
      (Utilities|FlowControl|Delay 3.0)
      (Actor|DestroyActor))))

(event EventBeginPlay
  (CallFunction|RandomSpawnDecor))

(event Collision|EventActorBeginOverlap
  (params (OtherActor :type Actor%20Object%20Reference)))

(event EventTick
  (params (DeltaSeconds :type Float%20%28single-precision%29)))

(fn ConstructionScript)

(fn RandomSpawnDecor
  (Utilities|FlowControl|Sequence
    (:then_0
      (Utilities|FlowControl|Sequence
        (:then_0
          (for _index (range 0 (Math|Random|RandomIntegerinRange (Variables|Default|GetMinRandomObstacleID) (Variables|Default|GetMaxRandomObstacleID)))
            (bind _returnfloats (CallFunction|GetFloatsfromBound (Variables|Default|GetTileFloorA)))
            (CallFunction|AddInstanceatLocation (Variables|Default|GetHierarchicalInstancedStaticMesh_TreeABody) _returnfloats)
            (CallFunction|AddInstanceatLocation (Variables|Default|GetHierarchicalInstancedStaticMesh_TreeAHead) _returnfloats)))
        (:then_1
          (for _index_2 (range 0 (Math|Random|RandomIntegerinRange (Variables|Default|GetMinRandomObstacleID) (Variables|Default|GetMaxRandomObstacleID)))
            (bind _returnfloats_2 (CallFunction|GetFloatsfromBound (Variables|Default|GetTileFloorA)))
            (CallFunction|AddInstanceatLocation (Variables|Default|GetHierarchicalInstancedStaticMesh_TreeBBody) _returnfloats_2)
            (CallFunction|AddInstanceatLocation (Variables|Default|GetHierarchicalInstancedStaticMesh_TreeBHead) _returnfloats_2)))
        (:then_2
          (for _index_3 (range 0 (Math|Random|RandomIntegerinRange 50 100))
            (bind _returnfloats_3 (CallFunction|GetFloatsfromBound (Variables|Default|GetTileFloorA)))
            (CallFunction|AddInstanceatLocation (Variables|Default|GetHierarchicalInstancedStaticMesh_Stump) (Math|Vector4|MakeVector4 (.X (Math|Vector4|BreakVector4 _returnfloats_3)) (.Y (Math|Vector4|BreakVector4 _returnfloats_3)) (.Z (Math|Vector4|BreakVector4 _returnfloats_3)) (* (.W (Math|Vector4|BreakVector4 _returnfloats_3)) 3.0)))))
        (:then_3
          (for _index_4 (range 0 (Math|Random|RandomIntegerinRange 999 1000))
            (bind _returnfloats_4 (CallFunction|GetFloatsfromBound (Variables|Default|GetTileFloorA)))
            (CallFunction|AddInstanceatLocation (Variables|Default|GetHierarchicalInstancedStaticMesh_Vegetation) (Math|Vector4|MakeVector4 (.X (Math|Vector4|BreakVector4 _returnfloats_4)) (.Y (Math|Vector4|BreakVector4 _returnfloats_4)) (.Z (Math|Vector4|BreakVector4 _returnfloats_4)) (* (.W (Math|Vector4|BreakVector4 _returnfloats_4)) 2.0)))))
        (:then_4
          (for _index_5 (range 0 (Math|Random|RandomIntegerinRange 1999 2000))
            (bind _returnfloats_5 (CallFunction|GetFloatsfromBound (Variables|Default|GetTileFloorA)))
            (CallFunction|AddInstanceatLocation (Variables|Default|GetHierarchicalInstancedStaticMesh_Vegetation3) (Math|Vector4|MakeVector4 (.X (Math|Vector4|BreakVector4 _returnfloats_5)) (.Y (Math|Vector4|BreakVector4 _returnfloats_5)) (.Z (Math|Vector4|BreakVector4 _returnfloats_5)) (* (.W (Math|Vector4|BreakVector4 _returnfloats_5)) 2.0)))))
        (:then_5
          (for _index_6 (range 0 (Math|Random|RandomIntegerinRange 800 1000))
            (bind _returnfloats_6 (CallFunction|GetFloatsfromBound (Variables|Default|GetTileFloorA)))
            (CallFunction|AddInstanceatLocation (Variables|Default|GetHierarchicalInstancedStaticMesh_Vegetation2) (Math|Vector4|MakeVector4 (.X (Math|Vector4|BreakVector4 _returnfloats_6)) (.Y (Math|Vector4|BreakVector4 _returnfloats_6)) (.Z (Math|Vector4|BreakVector4 _returnfloats_6)) (* (.W (Math|Vector4|BreakVector4 _returnfloats_6)) 2.0)))))))
    (:then_1
      (Utilities|FlowControl|Sequence
        (:then_0
          (for _index_7 (range 0 (Math|Random|RandomIntegerinRange 20 21))
            (bind _returnfloats_7 (CallFunction|GetFloatsfromBound (Variables|Default|GetTileFloorB)))
            (CallFunction|AddInstanceatLocation (Variables|Default|GetHierarchicalInstancedStaticMesh_TreeABody) _returnfloats_7)
            (CallFunction|AddInstanceatLocation (Variables|Default|GetHierarchicalInstancedStaticMesh_TreeAHead) _returnfloats_7)))
        (:then_1
          (for _index_8 (range 0 (Math|Random|RandomIntegerinRange 20 21))
            (bind _returnfloats_8 (CallFunction|GetFloatsfromBound (Variables|Default|GetTileFloorB)))
            (CallFunction|AddInstanceatLocation (Variables|Default|GetHierarchicalInstancedStaticMesh_TreeBBody) _returnfloats_8)
            (CallFunction|AddInstanceatLocation (Variables|Default|GetHierarchicalInstancedStaticMesh_TreeBHead) _returnfloats_8)))
        (:then_2
          (for _index_9 (range 0 (Math|Random|RandomIntegerinRange 5 10))
            (bind _returnfloats_9 (CallFunction|GetFloatsfromBound (Variables|Default|GetTileFloorB)))
            (CallFunction|AddInstanceatLocation (Variables|Default|GetHierarchicalInstancedStaticMesh_Stump) (Math|Vector4|MakeVector4 (.X (Math|Vector4|BreakVector4 _returnfloats_9)) (.Y (Math|Vector4|BreakVector4 _returnfloats_9)) (.Z (Math|Vector4|BreakVector4 _returnfloats_9)) (* (.W (Math|Vector4|BreakVector4 _returnfloats_9)) 3.0)))))
        (:then_3
          (for _index_10 (range 0 (Math|Random|RandomIntegerinRange 999 1000))
            (bind _returnfloats_10 (CallFunction|GetFloatsfromBound (Variables|Default|GetTileFloorB)))
            (CallFunction|AddInstanceatLocation (Variables|Default|GetHierarchicalInstancedStaticMesh_Vegetation) (Math|Vector4|MakeVector4 (.X (Math|Vector4|BreakVector4 _returnfloats_10)) (.Y (Math|Vector4|BreakVector4 _returnfloats_10)) (.Z (Math|Vector4|BreakVector4 _returnfloats_10)) (* (.W (Math|Vector4|BreakVector4 _returnfloats_10)) 2.0)))))
        (:then_4
          (for _index_11 (range 0 (Math|Random|RandomIntegerinRange 1999 2000))
            (bind _returnfloats_11 (CallFunction|GetFloatsfromBound (Variables|Default|GetTileFloorB)))
            (CallFunction|AddInstanceatLocation (Variables|Default|GetHierarchicalInstancedStaticMesh_Vegetation3) (Math|Vector4|MakeVector4 (.X (Math|Vector4|BreakVector4 _returnfloats_11)) (.Y (Math|Vector4|BreakVector4 _returnfloats_11)) (.Z (Math|Vector4|BreakVector4 _returnfloats_11)) (* (.W (Math|Vector4|BreakVector4 _returnfloats_11)) 2.0)))))
        (:then_5
          (for _index_12 (range 0 (Math|Random|RandomIntegerinRange 800 1000))
            (bind _returnfloats_12 (CallFunction|GetFloatsfromBound (Variables|Default|GetTileFloorB)))
            (CallFunction|AddInstanceatLocation (Variables|Default|GetHierarchicalInstancedStaticMesh_Vegetation2) (Math|Vector4|MakeVector4 (.X (Math|Vector4|BreakVector4 _returnfloats_12)) (.Y (Math|Vector4|BreakVector4 _returnfloats_12)) (.Z (Math|Vector4|BreakVector4 _returnfloats_12)) 0.0))))))
    (:then_3
      (Utilities|FlowControl|Sequence
        (:then_0
          (for _index_13 (range 0 (Math|Random|RandomIntegerinRange (Variables|Default|GetMinRandomObstacleID) (Variables|Default|GetMaxRandomObstacleID)))
            (bind _returnfloats_13 (CallFunction|GetFloatsfromBound (Variables|Default|GetTileFloorD)))
            (CallFunction|AddInstanceatLocation (Variables|Default|GetHierarchicalInstancedStaticMesh_TreeABody) _returnfloats_13)
            (CallFunction|AddInstanceatLocation (Variables|Default|GetHierarchicalInstancedStaticMesh_TreeAHead) _returnfloats_13)))
        (:then_1
          (for _index_14 (range 0 (Math|Random|RandomIntegerinRange (Variables|Default|GetMinRandomObstacleID) (Variables|Default|GetMaxRandomObstacleID)))
            (bind _returnfloats_14 (CallFunction|GetFloatsfromBound (Variables|Default|GetTileFloorD)))
            (CallFunction|AddInstanceatLocation (Variables|Default|GetHierarchicalInstancedStaticMesh_TreeBBody) _returnfloats_14)
            (CallFunction|AddInstanceatLocation (Variables|Default|GetHierarchicalInstancedStaticMesh_TreeBHead) _returnfloats_14)))
        (:then_2
          (for _index_15 (range 0 (Math|Random|RandomIntegerinRange (Variables|Default|GetMinRandomObstacleID) (Variables|Default|GetMaxRandomObstacleID)))
            (bind _returnfloats_15 (CallFunction|GetFloatsfromBound (Variables|Default|GetTileFloorD)))
            (CallFunction|AddInstanceatLocation (Variables|Default|GetHierarchicalInstancedStaticMesh_Stump) (Math|Vector4|MakeVector4 (.X (Math|Vector4|BreakVector4 _returnfloats_15)) (.Y (Math|Vector4|BreakVector4 _returnfloats_15)) (.Z (Math|Vector4|BreakVector4 _returnfloats_15)) (* (.W (Math|Vector4|BreakVector4 _returnfloats_15)) 3.0)))))
        (:then_3
          (for _index_16 (range 0 (Math|Random|RandomIntegerinRange 10 20))
            (bind _returnfloats_16 (CallFunction|GetFloatsfromBound (Variables|Default|GetTileFloorD)))
            (CallFunction|AddInstanceatLocation (Variables|Default|GetHierarchicalInstancedStaticMesh_Bark) (Math|Vector4|MakeVector4 (.X (Math|Vector4|BreakVector4 _returnfloats_16)) (.Y (Math|Vector4|BreakVector4 _returnfloats_16)) (.Z (Math|Vector4|BreakVector4 _returnfloats_16)) (* (.W (Math|Vector4|BreakVector4 _returnfloats_16)) 2.0)))))
        (:then_4
          (for _index_17 (range 0 (Math|Random|RandomIntegerinRange 999 1000))
            (bind _returnfloats_17 (CallFunction|GetFloatsfromBound (Variables|Default|GetTileFloorD)))
            (CallFunction|AddInstanceatLocation (Variables|Default|GetHierarchicalInstancedStaticMesh_Vegetation) (Math|Vector4|MakeVector4 (.X (Math|Vector4|BreakVector4 _returnfloats_17)) (.Y (Math|Vector4|BreakVector4 _returnfloats_17)) (.Z (Math|Vector4|BreakVector4 _returnfloats_17)) (* (.W (Math|Vector4|BreakVector4 _returnfloats_17)) 2.0)))))
        (:then_5
          (for _index_18 (range 0 (Math|Random|RandomIntegerinRange 1999 2000))
            (bind _returnfloats_18 (CallFunction|GetFloatsfromBound (Variables|Default|GetTileFloorD)))
            (CallFunction|AddInstanceatLocation (Variables|Default|GetHierarchicalInstancedStaticMesh_Vegetation3) (Math|Vector4|MakeVector4 (.X (Math|Vector4|BreakVector4 _returnfloats_18)) (.Y (Math|Vector4|BreakVector4 _returnfloats_18)) (.Z (Math|Vector4|BreakVector4 _returnfloats_18)) (* (.W (Math|Vector4|BreakVector4 _returnfloats_18)) 2.0)))))
        (:then_6
          (for _index_19 (range 0 (Math|Random|RandomIntegerinRange 800 1000))
            (bind _returnfloats_19 (CallFunction|GetFloatsfromBound (Variables|Default|GetTileFloorD)))
            (CallFunction|AddInstanceatLocation (Variables|Default|GetHierarchicalInstancedStaticMesh_Vegetation2) (Math|Vector4|MakeVector4 (.X (Math|Vector4|BreakVector4 _returnfloats_19)) (.Y (Math|Vector4|BreakVector4 _returnfloats_19)) (.Z (Math|Vector4|BreakVector4 _returnfloats_19)) 0.0))))))))

(fn GetFloatsfromBound
  (params (Component :type Scene%20Component%20Object%20Reference))
  (bind (_origin _boxextent) (Collision|GetComponentBounds Component))
  (bind (_x _y _z) (Math|Vector|BreakVector _boxextent))
  (bind _returnvalue (* _y 1.0))
  (bind _returnvalue_2 (Math|Vector|MakeVector _x _returnvalue _z))
  (bind _returnvalue_3 (Math|Random|RandomPointinBoundingBox _origin _returnvalue_2))
  (return (Math|Vector4|MakeVector4 (- (.x _returnvalue_3) (.x (Transformation|GetActorLocation))) (.y _returnvalue_3) (Math|Random|RandomFloatinRange 0.0 359.0) (Math|Random|RandomFloatinRange 0.8 1.2))))

(fn AddInstanceatLocation
  (params (InInstance :type Instanced%20Static%20Mesh%20Component%20Object%20Reference) (InFloats :type Vector%204%20Structure))
  (bind (_x _y _z _w) (Math|Vector4|BreakVector4 InFloats))
  (Components|InstancedStaticMesh|AddInstance InInstance (Math|Transform|MakeTransform (Math|Vector|MakeVector _x _y 0.0) (Math|Rotator|MakeRotator 0.0 0.0 _z) (Math|Vector|MakeVector _w _w _w))))