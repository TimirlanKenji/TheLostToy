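; BP_Plushe is an overlap pickup in the environment that counts as a coin for the third-person character.
; On overlap it calls the character's Dialogue, increments Coins on BP_ThirdPersonGameMode, spawns a star-trail emitter on its mesh with auto-activate off, then destroys itself.
; Unconnected leftover nodes would randomly rotate the mesh and put a knife mesh on BP_YippyCharacter's stick.
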(event EventBeginPlay)

(event EventTick
  (params (DeltaSeconds :type Float%20%28single-precision%29)))

(event Collision|EventActorBeginOverlap
  (params (OtherActor :type Actor%20Object%20Reference))
  (bind _asbp_third_person_character (Utilities|Casting|CastToBP_ThirdPersonCharacter OtherActor))
  ;[0.3144 1 0.2917] Call the DIALOGUE
  (Default|Dialogue _asbp_third_person_character)
  (bind _asbp_third_person_game_mode (Utilities|Casting|CastToBP_ThirdPersonGameMode (Game|GetGameMode)))
  (Math|Integer|IncrementInt (Variables|/Game/Blueprints/BP_ThirdPersonGameMode.BP_ThirdPersonGameMode_C|GetCoins _asbp_third_person_game_mode)
    (:%20%20
      (Effects|SpawnEmitterAttached "/Game/CartoonFX2/Particles/ExplosionParts/PS_TrailStars.PS_TrailStars" (Variables|Default|GetStaticMesh) "spine_03" (Transformation|GetWorldLocation (Variables|Default|GetDefaultSceneRoot)) "0, 0, 0" "1.000000,1.000000,1.000000" "KeepWorldPosition" false "None" false)
      ;[1 0.2071 0.3371] Destroy
      (Actor|DestroyActor))))

(fn ConstructionScript)